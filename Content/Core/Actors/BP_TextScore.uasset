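; BP_TextScore is an actor that displays the player's collected coin count as text rendered in the world.
; A looping timer started on BeginPlay polls CoinsCollected on BP_GameState instead of using Tick, and is cleared on EndPlay.
; UpdateCoins rebuilds the TextRender message only when the count differs from its cached CurrentCoinsCollected value.
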(event `self.ReceiveBeginPlay`
  (bind _returnvalue (`KismetSystemLibrary.K2_SetTimer` null "UpdateCoins" 0.5 true true 0.5 0.5))
  (set `self.TimerUpdateCoins` _returnvalue))

(event `self.ReceiveEndPlay`
  (params (EndPlayReason :type "EEndPlayReason Enum" :default "Destroyed"))
  (`KismetSystemLibrary.K2_ClearAndInvalidateTimerHandle` (`self.TimerUpdateCoins`)))

(fn `UpdateCoins`
  (bind _coinscollected (`/Game/Core/BP_GameState.CoinsCollected` (cast `/Game/Core/BP_GameState` (`GameplayStatics.GetGameState`) :!pure true)))
  (if (!= (`self.CurrentCoinsCollected`) _coinscollected)
    (`TextRenderComponent.K2_SetText` (`self.TextRender`) (`KismetTextLibrary.Conv_StringToText` (`KismetStringLibrary.Concat_StrStr` "You collected " (`KismetStringLibrary.Conv_IntToString` _coinscollected) " coins.")))
    (set `self.CurrentCoinsCollected` _coinscollected)))

(fn `UserConstructionScript`)