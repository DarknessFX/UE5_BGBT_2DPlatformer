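; BP_Platform_PingPong is a moving platform actor that, as its name suggests, travels back and forth.
; Tick offsets the root component along relative X by Speed scaled with delta time, using a swept move.
; An overlap with any actor other than the first player's pawn recomputes Speed from its current value, presumably flipping the direction, so the player does not trigger a turnaround.
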(event `self.ReceiveTick`
  (params (DeltaSeconds :type "Float (single-precision)"))
  (`SceneComponent.K2_AddRelativeLocation` (`self.DefaultSceneRoot`) (`KismetMathLibrary.MakeVector` (* DeltaSeconds (`self.Speed`))) true false))

(event `self.ReceiveActorBeginOverlap`
  (params (OtherActor :type "Actor Object Reference"))
  (if (!= OtherActor (`GameplayStatics.GetPlayerPawn` 0))
    (bind _result (`/Engine/EditorBlueprintResources/StandardMacros.NegateFloat` (`self.Speed`))
      (:`  `
        (set `self.Speed` _result)))))

(fn `UserConstructionScript`)