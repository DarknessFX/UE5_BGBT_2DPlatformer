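; BP_Enemy_Slime is a patrolling slime enemy that deals damage to the player on contact.
; Tick sweeps its flipbook along X by Speed, and FlipDirection updates Speed and rotates the sprite 180 degrees.
; It flips when either ground check stops overlapping a non-player actor, or when the flipbook begins overlapping one.
; Flipbook overlaps ignore coins, identified by "Coin" in the object name.
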(event `self.GroundCheckLeft.OnComponentEndOverlap`
  (params (OverlappedComponent :type "PrimitiveComponent Object Reference") (OtherActor :type "Actor Object Reference") (OtherComp :type "PrimitiveComponent Object Reference") (OtherBodyIndex :type Integer))
  (`self.IgnorePawn` OtherActor
    (:`True`
      (`self.FlipDirection`))))

(event `self.GroundCheckRight.OnComponentEndOverlap`
  (params (OverlappedComponent :type "PrimitiveComponent Object Reference") (OtherActor :type "Actor Object Reference") (OtherComp :type "PrimitiveComponent Object Reference") (OtherBodyIndex :type Integer))
  (`self.IgnorePawn` OtherActor
    (:`True`
      (`self.FlipDirection`))))

(event `self.ReceiveTick`
  (params (DeltaSeconds :type "Float (single-precision)"))
  (`SceneComponent.K2_AddRelativeLocation` (`self.PaperFlipbook`) (`KismetMathLibrary.MakeVector` (* DeltaSeconds (`self.Speed`))) true false))

(event `self.PaperFlipbook.OnComponentBeginOverlap`
  (params (OverlappedComponent :type "PrimitiveComponent Object Reference") (OtherActor :type "Actor Object Reference") (OtherComp :type "PrimitiveComponent Object Reference") (OtherBodyIndex :type Integer) (bFromSweep :type Boolean) (SweepResult :type "HitResult Structure (by ref)"))
  (`self.IgnorePawn` OtherActor
    (:`True`
      (`self.IgnoreCoins` OtherActor
        (:`True`
          (`self.FlipDirection`))))
    (:`False`
      (`GameplayStatics.ApplyDamage` (`GameplayStatics.GetPlayerPawn` 0) 1.0 null self "/Script/Engine.DamageType"))))

(fn `FlipDirection`
  (bind _result (`/Engine/EditorBlueprintResources/StandardMacros.NegateFloat` (`self.Speed`))
    (:`  `
      (set `self.Speed` _result)
      (`SceneComponent.K2_AddLocalRotation` (`self.PaperFlipbook`) (struct :`Yaw` 180.0) false false))))

(fn `UserConstructionScript`)