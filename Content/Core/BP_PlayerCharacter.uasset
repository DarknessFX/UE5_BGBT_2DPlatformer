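; Player-controlled 2D knight that runs and jumps along the X axis and collects coins into BP_GameState's counter, matching them by object name.
; Enhanced Input drives movement, while UpdateAnimation swaps idle, run and jump flipbooks and flips facing through control yaw.
; Any damage plays the hit flipbook, disables input and collision, and drops the body with physics in slow motion before destroying it.
; Destruction hands the view to a CameraActor, and EndPlay calls RestartLevel.
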(event `self.ReceiveEndPlay`
  (params (EndPlayReason :type "EEndPlayReason Enum" :default "Destroyed"))
  (`/Game/Core/BP_GameState.RestartLevel` (cast `/Game/Core/BP_GameState` (`GameplayStatics.GetGameState`) :!pure true)))

(event `self.ReceiveDestroyed`
  (bind _returnvalue (`GameplayStatics.GetActorOfClass` "/Script/Engine.CameraActor"))
  (`PlayerController.SetViewTargetWithBlend` (`GameplayStatics.GetPlayerController` 0) _returnvalue 0.0 "VTBlend_EaseInOut" 0.0 true))

(event `self.ReceivePossessed`
  (params (NewController :type "Controller Object Reference"))
  (message `EnhancedInputSubsystemInterface.AddMappingContext` (pcsubsystem `EnhancedInputLocalPlayerSubsystem` (cast `PlayerController` NewController :!pure true)) "/Game/Input/IMC_Player.IMC_Player" 0 (struct)))

(event `EnhancedInput|/Game/Input/Actions/IA_Jump`
  (params (ActionValue :type Boolean) (ElapsedSeconds :type "Float (double-precision)") (TriggeredSeconds :type "Float (double-precision)") (InputAction :type "InputAction Object Reference" :default "/Game/Input/Actions/IA_Jump.IA_Jump"))
  (:`Started`
    (`self.Jump`)
    (set `self.IsJumping` true)
    (`self.UpdateAnimation` 0.0)))

(event `self.OnLanded`
  (params (Hit :type "HitResult Structure (by ref)"))
  (`self.StopJumping`)
  (set `self.IsJumping` false)
  (`self.UpdateAnimation` 0.0))

(event `EnhancedInput|/Game/Input/Actions/IA_Move`
  (params (ActionValue :type "Float (double-precision)") (ElapsedSeconds :type "Float (double-precision)") (TriggeredSeconds :type "Float (double-precision)") (InputAction :type "InputAction Object Reference" :default "/Game/Input/Actions/IA_Move.IA_Move"))
  (:`Triggered`
    (`self.AddMovementInput` (1.0 0.0 0.0) ActionValue)
    (`self.UpdateAnimation` ActionValue :!label _label))
  (:`Completed`
    (goto _label)))

(event `self.ReceiveActorBeginOverlap`
  (params (OtherActor :type "Actor Object Reference"))
  (if (`KismetStringLibrary.Contains` (`KismetSystemLibrary.GetObjectName` OtherActor) "Coin")
    (`self.K2_DestroyActor` OtherActor)
    (`/Engine/EditorBlueprintResources/StandardMacros.IncrementInt` (`/Game/Core/BP_GameState.CoinsCollected` (cast `/Game/Core/BP_GameState` (`GameplayStatics.GetGameState`) :!pure true)))))

(event `self.ReceiveAnyDamage`
  (params (Damage :type "Float (single-precision)") (DamageType :type "DamageType Object Reference") (InstigatedBy :type "Controller Object Reference") (DamageCauser :type "Actor Object Reference"))
  (bind _sprite (`self.Sprite`))
  (bind _capsulecomponent (`self.CapsuleComponent`))
  (`|ExecutionSequence`
    (:`then_0`
      (`PaperFlipbookComponent.SetLooping` _sprite false)
      (`PaperFlipbookComponent.SetFlipbook` _sprite "/Game/Assets/Flipbooks/FB_Knight_Hit.FB_Knight_Hit")
      (`self.DisableInput` (`GameplayStatics.GetPlayerController` 0)))
    (:`then_1`
      (`self.SetActorEnableCollision` self false)
      (`PrimitiveComponent.SetCollisionEnabled` _capsulecomponent "NoCollision")
      (`PrimitiveComponent.SetCollisionEnabled` (`self.Sprite`) "NoCollision")
      (`PrimitiveComponent.SetSimulatePhysics` _capsulecomponent true)
      (`PrimitiveComponent.SetSimulatePhysics` (`self.Sprite`) true))
    (:`then_2`
      (`GameplayStatics.SetGlobalTimeDilation` 0.5)
      (`KismetSystemLibrary.Delay` 1.0)
      (`self.K2_DestroyActor` self))))

(fn `UpdateAnimation`
  (params (Input :type "Float (double-precision)"))
  (locals (NextFlipbook :type "PaperFlipbook Object Reference" :default "/Script/Paper2D.PaperFlipbook'/Game/Assets/Flipbooks/FB_Knight_Jump.FB_Knight_Jump'"))
  (bind _returnvalue (`self.GetController`))
  (bind _sprite (`self.Sprite`))
  (bind _nextflipbook (`local.NextFlipbook`))
  (`|ExecutionSequence`
    (:`then_0`
      (if (`self.IsJumping`)
        (set `local.NextFlipbook` "/Game/Assets/Flipbooks/FB_Knight_Jump.FB_Knight_Jump")
        (else
          (`/Engine/EditorBlueprintResources/StandardMacros.CompareFloat` Input
            (:`>`
              (set `local.NextFlipbook` "/Game/Assets/Flipbooks/FB_Knight_Run.FB_Knight_Run" :!label _label))
            (:`==`
              (set `local.NextFlipbook` "/Game/Assets/Flipbooks/FB_Knight_Idle.FB_Knight_Idle"))
            (:`<`
              (goto _label))))))
    (:`then_1`
      (if (!= (`PaperFlipbookComponent.GetFlipbook` _sprite) _nextflipbook)
        (`PaperFlipbookComponent.SetFlipbook` _sprite _nextflipbook)))
    (:`then_2`
      (`/Engine/EditorBlueprintResources/StandardMacros.CompareFloat` Input
        (:`>`
          (`Controller.SetControlRotation` _returnvalue (`KismetMathLibrary.MakeRotator` 0.0)))
        (:`<`
          (`Controller.SetControlRotation` _returnvalue (`KismetMathLibrary.MakeRotator` 0.0 0.0 180.0)))))))

(fn `UserConstructionScript`)